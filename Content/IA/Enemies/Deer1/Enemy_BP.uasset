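; Enemy Blueprint (Deer1) that wanders around its spawn point and chases actors tagged Player or Pet.
; Tick accumulates time while stationary, then sends it to a random patrol point unless it is detecting or attacking.
; Detection overlap sets the target and starts AIMoveTo, while attack overlap only toggles IsAttacking.
; HitEnemy, not called in this graph, damages MyCharacter_BP or lobo_BP; ApplyDamage lowers HP and briefly flags IsHitted, without death handling.
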(event `self.ReceiveBeginPlay`
  (set `self.initialPosition` (`SceneComponent.K2_GetComponentLocation` (`self.RootComponent`))))

(event `self.ReceiveTick`
  (params (DeltaSeconds :type "Float (single-precision)"))
  (bind _idle_time (`self.calculateIdleTime` DeltaSeconds))
  (bind _output_get (set `self.idleTime` _idle_time))
  (if (and (> _output_get 5.0) (!= (`self.isAttacking`) true) (!= (`self.isDetecting`) true))
    (bind _returnvalue (`self.getRandomTarget`))
    (`|AIMoveTo` self _returnvalue null
      (:`then`
        (set `self.idleTime` 0.0)))))

(event `self.RadiusDetection.OnComponentBeginOverlap`
  (params (OverlappedComponent :type "PrimitiveComponent Object Reference") (OtherActor :type "Actor Object Reference") (OtherComp :type "PrimitiveComponent Object Reference") (OtherBodyIndex :type Integer) (bFromSweep :type Boolean) (SweepResult :type "HitResult Structure (by ref)"))
  (if (or (`self.ActorHasTag` OtherActor "Pet") (`self.ActorHasTag` OtherActor "Player"))
    (set `self.TargetEnemy` OtherActor)
    (set `self.isDetecting` true)
    (`self.Follow Enemy`)))

(event `self.RadiusDetection.OnComponentEndOverlap`
  (params (OverlappedComponent :type "PrimitiveComponent Object Reference") (OtherActor :type "Actor Object Reference") (OtherComp :type "PrimitiveComponent Object Reference") (OtherBodyIndex :type Integer))
  (if (or (`self.ActorHasTag` OtherActor "Pet") (`self.ActorHasTag` OtherActor "Player"))
    (set `self.TargetEnemy` null)
    (set `self.isDetecting` false)))

(event `self.RadiusAttack.OnComponentBeginOverlap`
  (params (OverlappedComponent :type "PrimitiveComponent Object Reference") (OtherActor :type "Actor Object Reference") (OtherComp :type "PrimitiveComponent Object Reference") (OtherBodyIndex :type Integer) (bFromSweep :type Boolean) (SweepResult :type "HitResult Structure (by ref)"))
  (if (or (`self.ActorHasTag` OtherActor "Pet") (`self.ActorHasTag` OtherActor "Player"))
    (set `self.isAttacking` true)))

(event `self.RadiusAttack.OnComponentEndOverlap`
  (params (OverlappedComponent :type "PrimitiveComponent Object Reference") (OtherActor :type "Actor Object Reference") (OtherComp :type "PrimitiveComponent Object Reference") (OtherBodyIndex :type Integer))
  (if (or (`self.ActorHasTag` OtherActor "Pet") (`self.ActorHasTag` OtherActor "Player"))
    (set `self.isAttacking` false)))

(event `Follow Enemy`
  (if (and (!= (`self.isAttacking`) true) (`self.isDetecting`))
    (`|AIMoveTo` self (0.0 0.0 0.0) (`self.TargetEnemy`) 5.0 true)))

(event `Hit Enemy`
  (bind _targetenemy (`self.TargetEnemy`))
  (bind _damage (`self.damage`))
  (if (`self.ActorHasTag` _targetenemy "Player")
    (bind _asmy_character_bp (cast `/Game/Characters/MyCharacter_BP` (`self.TargetEnemy`)))
    (`/Game/Characters/MyCharacter_BP.Apply Damage` _asmy_character_bp _damage)
    (elif (`self.ActorHasTag` _targetenemy "Pet")
      (bind _aslobo_bp (cast `/Game/IA/Secuaces/Lobo/lobo_BP` (`self.TargetEnemy`)))
      (`/Game/IA/Secuaces/Lobo/lobo_BP.ApplyDamage` _aslobo_bp _damage))))

(event `ApplyDamage`
  (params (Damage :type "Float (double-precision)"))
  (set `self.HP` (- (`self.HP`) Damage))
  (set `self.isHitted` true)
  (`KismetSystemLibrary.Delay` 0.2)
  (set `self.isHitted` false))

(fn `calculateIdleTime`
  (params (`Delta Seconds` :type "Float (double-precision)"))
  (returns (`idle Time` :type "Float (double-precision)"))
  (if (== (`KismetMathLibrary.VSize` (`self.GetVelocity`)) 0.0)
    (return (+ `Delta Seconds` (`self.idleTime`)))
    (else
      (return 0.0))))

(fn `getRandomTarget`
  (returns (ReturnValue :type "Vector Structure"))
  (bind _patroldistance (`self.PatrolDistance`))
  (bind _initialposition (`self.initialPosition`))
  (bind _returnvalue (+ _initialposition (`KismetMathLibrary.MakeVector` (`KismetMathLibrary.RandomFloatInRange` (* -1 _patroldistance) _patroldistance) (`KismetMathLibrary.RandomFloatInRange` (* -1 _patroldistance) _patroldistance))))
  (`KismetSystemLibrary.PrintString` (`KismetStringLibrary.Concat_StrStr` (`KismetStringLibrary.Conv_VectorToString` _initialposition) " a " (`KismetStringLibrary.Conv_VectorToString` _returnvalue)) true true (struct :`G` 0.66 :`B` 1.0 :`A` 1.0) 10.0)
  (return _returnvalue))

(fn `UserConstructionScript`)