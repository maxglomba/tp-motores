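; Enemy actor that detects, chases and damages the player or their pet.
; Two overlap radii filter by Player and Pet tags to set the target plus detecting and attacking flags.
; FollowEnemy moves toward the target until in attack range, and HitEnemy casts it to the character or wolf Blueprint to deal damage, both triggered externally.
; ApplyDamage lowers HP and briefly raises a hit flag, with no death handling here.
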(event `self.RadiusDetection.OnComponentBeginOverlap`
  (params (OverlappedComponent :type "PrimitiveComponent Object Reference") (OtherActor :type "Actor Object Reference") (OtherComp :type "PrimitiveComponent Object Reference") (OtherBodyIndex :type Integer) (bFromSweep :type Boolean) (SweepResult :type "HitResult Structure (by ref)"))
  (if (or (`self.ActorHasTag` OtherActor "Pet") (`self.ActorHasTag` OtherActor "Player"))
    (set `self.TargetEnemy` OtherActor)
    (set `self.isDetecting` true)))

(event `self.RadiusDetection.OnComponentEndOverlap`
  (params (OverlappedComponent :type "PrimitiveComponent Object Reference") (OtherActor :type "Actor Object Reference") (OtherComp :type "PrimitiveComponent Object Reference") (OtherBodyIndex :type Integer))
  (if (or (`self.ActorHasTag` OtherActor "Pet") (`self.ActorHasTag` OtherActor "Player"))
    (set `self.TargetEnemy` null)
    (set `self.isDetecting` false)))

(event `self.RadiusAttack.OnComponentBeginOverlap`
  (params (OverlappedComponent :type "PrimitiveComponent Object Reference") (OtherActor :type "Actor Object Reference") (OtherComp :type "PrimitiveComponent Object Reference") (OtherBodyIndex :type Integer) (bFromSweep :type Boolean) (SweepResult :type "HitResult Structure (by ref)"))
  (if (or (`self.ActorHasTag` OtherActor "Pet") (`self.ActorHasTag` OtherActor "Player"))
    (set `self.isAttacking` true)))

(event `self.RadiusAttack.OnComponentEndOverlap`
  (params (OverlappedComponent :type "PrimitiveComponent Object Reference") (OtherActor :type "Actor Object Reference") (OtherComp :type "PrimitiveComponent Object Reference") (OtherBodyIndex :type Integer))
  (if (or (`self.ActorHasTag` OtherActor "Pet") (`self.ActorHasTag` OtherActor "Player"))
    (set `self.isAttacking` false)))

(event `Follow Enemy`
  (if (and (!= (`self.isAttacking`) true) (`self.isDetecting`))
    (`|AIMoveTo` null (0.0 0.0 0.0) (`self.TargetEnemy`) 5.0 true)))

(event `Hit Enemy`
  (bind _targetenemy (`self.TargetEnemy`))
  (bind _damage (`self.damage`))
  (if (`self.ActorHasTag` _targetenemy "Player")
    (bind _asmy_character_bp (cast `/Game/Characters/MyCharacter_BP` (`self.TargetEnemy`)))
    (`/Game/Characters/MyCharacter_BP.Apply Damage` _asmy_character_bp _damage)
    (elif (`self.ActorHasTag` _targetenemy "Pet")
      (bind _aslobo_bp (cast `/Game/IA/Secuaces/Lobo/lobo_BP` (`self.TargetEnemy`)))
      (`/Game/IA/Secuaces/Lobo/lobo_BP.ApplyDamage` _aslobo_bp _damage))))

(event `ApplyDamage`
  (params (Damage :type "Float (double-precision)"))
  (set `self.HP` (- (`self.HP`) Damage))
  (set `self.isHitted` true)
  (`KismetSystemLibrary.Delay` 0.2)
  (set `self.isHitted` false))

(fn `UserConstructionScript`)