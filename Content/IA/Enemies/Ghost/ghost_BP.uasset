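; Ghost enemy that patrols a looping list of walk points and damages player characters entering its attack area.
; Tick drives AIMoveTo between points, or halts movement while attacking and reapplies damage periodically; attacks end on overlap exit or depleted Sanity.
; While walking, it periodically traces down to spawn footprints, flagged visible when the local pawn is not MyCharacter_BP.
; Separate events toggle mesh visibility, and construction places it on the route.
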(event `self.ReceiveTick`
  (params (DeltaSeconds :type "Float (single-precision)"))
  (bind _targetactor (`self.targetActor`))
  (bind _charactermovement (`self.CharacterMovement`))
  (`self.doStep`)
  (if (!= (`self.isAttacking`) true)
    (set `self.walkingTime` (+ (`self.walkingTime`) DeltaSeconds))
    (`CharacterMovementComponent.SetMovementMode` _charactermovement "MOVE_Walking" 0)
    (`|AIMoveTo` self (0.0 0.0 0.0) (`self.currentTarget`)
      (:`OnSuccess`
        (`/Engine/EditorBlueprintResources/StandardMacros.DoOnce` false :!label _label
          (:`Completed`
            (`self.getNextWalkPoint`)
            (`KismetSystemLibrary.Delay` 2.0)
            (goto _label :!via `Reset`)))))
    (else
      (set `self.walkingTime` 0.0)
      (`CharacterMovementComponent.DisableMovement` _charactermovement)
      (bind _output_get (set `self.attackTime` (+ (`self.attackTime`) DeltaSeconds)))
      (if (>= _output_get 2.5)
        (`/Game/Characters/MyCharacter_BP.Apply Damage` _targetactor (`self.damage`))
        (set `self.attackTime` 0.0)
        (if (<= (`/Game/Characters/MyCharacter_BP.Sanity` _targetactor) 0.0)
          (set `self.isAttacking` false))))))

(event `changeVisibility`
  (params (visible :type Boolean))
  (`SceneComponent.SetVisibility` (`self.Mesh`) visible false))

(event `doStep`
  (bind _returnvalue (`self.K2_GetActorLocation`))
  (if (and (>= (`self.walkingTime`) 5.0) (== (`self.isAttacking`) false))
    (set `self.walkingTime` 0.0)
    (bind _outhit (`KismetSystemLibrary.LineTraceSingle` _returnvalue (- _returnvalue (0.0 0.0 500.0)) "TraceTypeQuery1"))
    (bind (_bblockinghit _binitialoverlap _time _distance _location _impactpoint) (`GameplayStatics.BreakHitResult` _outhit))
    (if _bblockinghit
      (cast `/Game/Characters/MyCharacter_BP` (`GameplayStatics.GetPlayerPawn` 0)
        (:`then`
          (bind _returnvalue_2 (`KismetMathLibrary.MakeTransform` (+ _impactpoint (0.0 0.0 5.0)) (`self.K2_GetActorRotation`) (2.0 2.0 1.0)))
          (`|SpawnActorFromClass` "/Game/Blueprints/footstep_BP.footstep_BP_C" _returnvalue_2 "AlwaysSpawn" "OverrideRootScale" null false null))
        (:`CastFailed`
          (`|SpawnActorFromClass` "/Game/Blueprints/footstep_BP.footstep_BP_C" _returnvalue_2 "AlwaysSpawn" "OverrideRootScale" null true null))))))

(event `self.AttackArea.OnComponentBeginOverlap`
  (params (OverlappedComponent :type "PrimitiveComponent Object Reference") (OtherActor :type "Actor Object Reference") (OtherComp :type "PrimitiveComponent Object Reference") (OtherBodyIndex :type Integer) (bFromSweep :type Boolean) (SweepResult :type "HitResult Structure (by ref)"))
  (bind _asmy_character_bp (cast `/Game/Characters/MyCharacter_BP` OtherActor))
  (set `self.targetActor` _asmy_character_bp)
  (set `self.isAttacking` true)
  (`/Game/Characters/MyCharacter_BP.Apply Damage` _asmy_character_bp (`self.damage`))
  (if (<= (`/Game/Characters/MyCharacter_BP.Sanity` _asmy_character_bp) 0.0)
    (set `self.isAttacking` false)))

(event `self.AttackArea.OnComponentEndOverlap`
  (params (OverlappedComponent :type "PrimitiveComponent Object Reference") (OtherActor :type "Actor Object Reference") (OtherComp :type "PrimitiveComponent Object Reference") (OtherBodyIndex :type Integer))
  (cast `/Game/Characters/MyCharacter_BP` OtherActor)
  (set `self.isAttacking` false))

(event `setGhostVisibility`
  (params (Visibility :type Boolean))
  (bind _mesh (`self.Mesh`))
  (if Visibility
    (`SceneComponent.SetVisibility` _mesh true false)
    (else
      (`SceneComponent.SetVisibility` _mesh false false))))

(fn `getNextWalkPoint`
  (bind _walkpoints (`self.walkPoints`))
  (if (`KismetSystemLibrary.IsValid` (`self.currentTarget`))
    (for (_array_element _array_index) _walkpoints
      (if (== (`self.currentTarget`) _array_element)
        (bind _returnvalue (+ _array_index 1))
        (if (<= _returnvalue (- (`KismetArrayLibrary.Array_Length` _walkpoints) 1))
          (set `self.targetIndex` _returnvalue)
          (set `self.currentTarget` (`|GetArrayItem` (`self.walkPoints`) _returnvalue))
          (break)
          (else
            (set `self.currentTarget` (`|GetArrayItem` (`self.walkPoints`)))
            (break)))))
    (`KismetSystemLibrary.PrintString` (`KismetStringLibrary.Conv_IntToString` (`self.targetIndex`)))
    (else
      (bind _output_get (set `self.targetIndex` 0))
      (set `self.currentTarget` (`|GetArrayItem` (`self.walkPoints`) _output_get)))))

(fn `UserConstructionScript`
  (`self.getNextWalkPoint`)
  (`self.K2_SetActorLocation` (`self.K2_GetActorLocation` (`self.currentTarget`)))
  (`self.getNextWalkPoint`))