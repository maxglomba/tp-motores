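; Deer enemy AI Blueprint with helpers for random patrol points and idle timing.
; GetRandomTarget picks a random XY offset within PatrolDistance of InitialPosition and debug-prints positions; CalculateIdleTime returns accumulated time while velocity is zero.
; All event entry points are empty.
; Disconnected, never-run logic would use detection and attack radius overlaps with Player or Pet actors to set target, state flags and a detection Blackboard key.
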(event `self.ReceiveBeginPlay`)

(event `self.ReceiveTick`
  (params (DeltaSeconds :type "Float (single-precision)")))

(event `self.RadiusDetection.OnComponentBeginOverlap`
  (params (OverlappedComponent :type "PrimitiveComponent Object Reference") (OtherActor :type "Actor Object Reference") (OtherComp :type "PrimitiveComponent Object Reference") (OtherBodyIndex :type Integer) (bFromSweep :type Boolean) (SweepResult :type "HitResult Structure (by ref)")))

(event `self.RadiusDetection.OnComponentEndOverlap`
  (params (OverlappedComponent :type "PrimitiveComponent Object Reference") (OtherActor :type "Actor Object Reference") (OtherComp :type "PrimitiveComponent Object Reference") (OtherBodyIndex :type Integer)))

(event `self.RadiusAttack.OnComponentBeginOverlap`
  (params (OverlappedComponent :type "PrimitiveComponent Object Reference") (OtherActor :type "Actor Object Reference") (OtherComp :type "PrimitiveComponent Object Reference") (OtherBodyIndex :type Integer) (bFromSweep :type Boolean) (SweepResult :type "HitResult Structure (by ref)")))

(event `self.RadiusAttack.OnComponentEndOverlap`
  (params (OverlappedComponent :type "PrimitiveComponent Object Reference") (OtherActor :type "Actor Object Reference") (OtherComp :type "PrimitiveComponent Object Reference") (OtherBodyIndex :type Integer)))

(fn `calculateIdleTime`
  (params (`Delta Seconds` :type "Float (double-precision)"))
  (returns (`idle Time` :type "Float (double-precision)"))
  (if (== (`KismetMathLibrary.VSize` (`self.GetVelocity`)) 0.0)
    (return (+ `Delta Seconds` (`self.idleTime`)))
    (else
      (return 0.0))))

(fn `getRandomTarget`
  (returns (ReturnValue :type "Vector Structure"))
  (bind _patroldistance (`self.PatrolDistance`))
  (bind _initialposition (`self.initialPosition`))
  (bind _returnvalue (+ _initialposition (`KismetMathLibrary.MakeVector` (`KismetMathLibrary.RandomFloatInRange` (* -1 _patroldistance) _patroldistance) (`KismetMathLibrary.RandomFloatInRange` (* -1 _patroldistance) _patroldistance))))
  (`KismetSystemLibrary.PrintString` (`KismetStringLibrary.Concat_StrStr` (`KismetStringLibrary.Conv_VectorToString` _initialposition) " a " (`KismetStringLibrary.Conv_VectorToString` _returnvalue)) true true (struct :`G` 0.66 :`B` 1.0 :`A` 1.0) 10.0)
  (return _returnvalue))

(fn `UserConstructionScript`)