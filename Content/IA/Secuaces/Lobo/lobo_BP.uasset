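; Wolf companion (lobo) AI that becomes the player's pet on proximity and follows them.
; Tick drives AI MoveTo following and flags sleep after idling.
; Detection and attack overlap volumes target tagged enemies and set attack state; it chases enemies only when not following the player.
; Events handle move orders, toggles, damage with a brief hit flag, and DataTable-based food healing; HitEnemy only casts the target, dealing no damage.
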(event `self.ReceiveTick`
  (params (DeltaSeconds :type "Float (single-precision)"))
  ;[1 0.7129 0.3326] Comment
  (`self.EvaluateSleep` DeltaSeconds)
  (if (`self.followPlayer`)
    (`|AIMoveTo` self (0.0 0.0 0.0) (`GameplayStatics.GetPlayerController` 0) 500.0)))

(event `EvaluateSleep`
  (params (EvaluateSleep :type "Float (double-precision)"))
  ;[1 0.7883 0.4354] Evaluate Sleep
  (if (== (`KismetMathLibrary.VSize` (`self.GetVelocity`)) 0.0)
    (set `self.idleTime` (+ (`self.idleTime`) EvaluateSleep))
    (if (> (`self.idleTime`) 5.0)
      (set `self.isSleeping` true))
    (else
      (set `self.idleTime` 0.0)
      (set `self.isSleeping` false))))

(event `Change Follow Player`
  ;[1 0.2422 0.1625] Cahnge Follow Player
  (set `self.followPlayer` (not (`self.followPlayer`))))

(event `Change Attack`
  ;[1 0.2837 0.1437] Change Attack
  (set `self.isAttacking` (not (`self.isAttacking`))))

(event `Go To Position`
  (params (Destination :type "Vector Structure") (AcceptanceRadius :type "Float (double-precision)"))
  ;[1 0.6623 0.1292] Go to Position
  (`|AIMoveTo` null Destination null AcceptanceRadius true))

(event `HealWithFood`
  (params (Name :type String))
  (bind _food_dt (`self.Food_DT`))
  ;[1 0.6105 0.09279] Heal With Food
  (bind _outrownames (`DataTableFunctionLibrary.GetDataTableRowNames` _food_dt))
  (for _array_element _outrownames
    (bind _returnvalue (`|GetDataTableRow` _food_dt _array_element)
      (:`then`
        (bind (_class _hprecovery _name) (break `/Game/Data/Food` _returnvalue))
        (if (`KismetStringLibrary.EqualEqual_StrStr` Name _name)
          (`self.Heal` _hprecovery)
          (break))))))

(event `Heal`
  (params (HP :type "Float (double-precision)"))
  ;[1 0.6105 0.09279] Heal
  (set `self.HP` (+ (`self.HP`) HP)))

(event `self.RadiusDetection.OnComponentBeginOverlap`
  (params (OverlappedComponent :type "PrimitiveComponent Object Reference") (OtherActor :type "Actor Object Reference") (OtherComp :type "PrimitiveComponent Object Reference") (OtherBodyIndex :type Integer) (bFromSweep :type Boolean) (SweepResult :type "HitResult Structure (by ref)"))
  (if (`self.ActorHasTag` OtherActor "Player")
    (bind _asmy_character_bp (cast `/Game/Characters/MyCharacter_BP` OtherActor))
    (cast `/Game/IA/Secuaces/Lobo/lobo_BP` (`/Game/Characters/MyCharacter_BP.Pet` _asmy_character_bp)
      (:`CastFailed`
        (set `/Game/Characters/MyCharacter_BP.Pet` self _asmy_character_bp)
        (set `self.followPlayer` true)))
    (elif (`self.ActorHasTag` OtherActor "Enemy")
      (set `self.detectingEnemy` true)
      (bind _output_get (set `self.enemyTargeted` OtherActor))
      (`self.Follow Enemy` _output_get))))

(event `self.RadiusDetection.OnComponentEndOverlap`
  (params (OverlappedComponent :type "PrimitiveComponent Object Reference") (OtherActor :type "Actor Object Reference") (OtherComp :type "PrimitiveComponent Object Reference") (OtherBodyIndex :type Integer))
  (if (`self.ActorHasTag` OtherActor "Enemy")
    (set `self.detectingEnemy` false)
    (set `self.enemyTargeted` null)))

(event `self.RadiusAttack.OnComponentBeginOverlap`
  (params (OverlappedComponent :type "PrimitiveComponent Object Reference") (OtherActor :type "Actor Object Reference") (OtherComp :type "PrimitiveComponent Object Reference") (OtherBodyIndex :type Integer) (bFromSweep :type Boolean) (SweepResult :type "HitResult Structure (by ref)"))
  (if (`self.ActorHasTag` OtherActor "Enemy")
    (set `self.isAttacking` true)))

(event `self.RadiusAttack.OnComponentEndOverlap`
  (params (OverlappedComponent :type "PrimitiveComponent Object Reference") (OtherActor :type "Actor Object Reference") (OtherComp :type "PrimitiveComponent Object Reference") (OtherBodyIndex :type Integer))
  (if (`self.ActorHasTag` OtherActor "Enemy")
    (set `self.isAttacking` false)))

(event `Follow Enemy`
  (params (TargetActor :type "Actor Object Reference"))
  (if (and (`self.detectingEnemy`) (not (`self.followPlayer`)))
    (`|AIMoveTo` null (0.0 0.0 0.0) TargetActor 5.0 true)))

(event `HitEnemy`
  (cast `/Game/IA/Enemies/Deer1/Enemy_BP` (`self.enemyTargeted`)))

(event `ApplyDamage`
  (params (Damage :type "Float (double-precision)"))
  (set `self.HP` (- (`self.HP`) Damage))
  (set `self.isHitted` true)
  (`KismetSystemLibrary.Delay` 0.2)
  (set `self.isHitted` false))

(fn `UserConstructionScript`)