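; Final door actor that shows a code menu to the player while their character stands in its trigger box.
; Box overlap begin and end cast to MyCharacter_BP, then tell its MyPlayerController_BP to turn the code menu status on or off.
; Two DoOnce gates re-arm each other, so show and hide alternate instead of repeating.
; The door itself has no opening or code-checking logic in these graphs.
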(event `self.Box.OnComponentBeginOverlap`
  (params (OverlappedComponent :type "PrimitiveComponent Object Reference") (OtherActor :type "Actor Object Reference") (OtherComp :type "PrimitiveComponent Object Reference") (OtherBodyIndex :type Integer) (bFromSweep :type Boolean) (SweepResult :type "HitResult Structure (by ref)"))
  (bind _asmy_character_bp (cast `/Game/Characters/MyCharacter_BP` OtherActor))
  (`/Engine/EditorBlueprintResources/StandardMacros.DoOnce` false :!label _label
    (:`Completed`
      (bind _asmy_player_controller_bp (cast `/Game/Blueprints/MyPlayerController_BP` (`Pawn.GetController` _asmy_character_bp)))
      (`/Game/Blueprints/MyPlayerController_BP.SetStatusCodeMenu` _asmy_player_controller_bp true)
      (goto _label_2 :!via `Reset`))))

(event `self.Box.OnComponentEndOverlap`
  (params (OverlappedComponent :type "PrimitiveComponent Object Reference") (OtherActor :type "Actor Object Reference") (OtherComp :type "PrimitiveComponent Object Reference") (OtherBodyIndex :type Integer))
  (bind _asmy_character_bp (cast `/Game/Characters/MyCharacter_BP` OtherActor))
  (`/Engine/EditorBlueprintResources/StandardMacros.DoOnce` false :!label _label_2
    (:`Completed`
      (bind _asmy_player_controller_bp (cast `/Game/Blueprints/MyPlayerController_BP` (`Pawn.GetController` _asmy_character_bp)))
      (`/Game/Blueprints/MyPlayerController_BP.SetStatusCodeMenu` _asmy_player_controller_bp false)
      (goto _label :!via `Reset`))))

(fn `UserConstructionScript`)