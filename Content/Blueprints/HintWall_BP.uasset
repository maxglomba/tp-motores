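; HintWall_BP is a hint wall actor that displays a text hint whose visibility can be switched on and off.
; SwitchTextVision shows or hides the TextRender and Plane components together, without propagating to their children.
; setTextHint converts the passed hint to text and writes it to the TextRender.
; It has no active BeginPlay, overlap or Tick logic and an empty construction script.
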(event `SwitchTextVision`
  (params (Enable :type Boolean))
  (bind _plane (`self.Plane`))
  (bind _textrender (`self.TextRender`))
  ;[0.5 0 0.03405] Text Vision
  (if Enable
    (`SceneComponent.SetVisibility` _textrender true false)
    (`SceneComponent.SetVisibility` _plane true false)
    (else
      (`SceneComponent.SetVisibility` _textrender false false)
      (`SceneComponent.SetVisibility` _plane false false))))

(event `setTextHint`
  (params (textHint :type String))
  (`TextRenderComponent.K2_SetText` (`self.TextRender`) (`KismetTextLibrary.Conv_StringToText` textHint)))

(fn `UserConstructionScript`)