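; Player controller that owns the game's UI: HUD, door code keypad, temporary messages and exit menu.
; BeginPlay creates the widgets; events show or hide the code and exit menus, switching input mode, cursor and MyCharacter_BP's StopMovement.
; The exit menu, opened by the OpenMenu input, also pauses the game, while messages appear only if none is showing.
; Restart restores game input, unpauses and reloads the current level, accepting normal or Soul pawns.
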(event `self.ReceiveBeginPlay`
  ;[1 0.7692 0.1892] BEGIN PLAY
  (bind _returnvalue (`|CreateWidget` "/Game/Interface/HUD_WBP.HUD_WBP_C" (`GameplayStatics.GetPlayerController` 0)))
  (bind _output_get (set `self.HUD` _returnvalue))
  (`UserWidget.AddToViewport` _output_get 0)
  (bind _returnvalue_2 (`|CreateWidget` "/Game/Interface/DoorCode_WBP.DoorCode_WBP_C"))
  (set `self.DoorCode_WID` _returnvalue_2)
  (set `self.openedDoorCode` false)
  (bind _returnvalue_3 (`|CreateWidget` "/Game/Interface/temporalMessage.temporalMessage_C"))
  (set `self.temporalMessage_WID` _returnvalue_3)
  (bind _returnvalue_4 (`|CreateWidget` "/Game/Interface/ExitMenu_WBP.ExitMenu_WBP_C"))
  (set `self.exiteMenu` _returnvalue_4))

(event `SetStatusCodeMenu`
  (params (Status :type Boolean))
  (bind _returnvalue (`GameplayStatics.GetPlayerController` 0))
  (bind _returnvalue_2 (`GameplayStatics.GetPlayerPawn` 0))
  (bind _doorcode_wid (`self.DoorCode_WID`))
  ;[0.5885 0 0] KeyCodeMenu
  (bind _output_get (set `self.openedDoorCode` Status))
  (if _output_get
    (`UserWidget.AddToViewport` _doorcode_wid 0)
    (`WidgetBlueprintLibrary.SetInputMode_UIOnlyEx` _returnvalue _doorcode_wid)
    (set `self.bShowMouseCursor` true)
    (bind _asmy_character_bp (cast `/Game/Characters/MyCharacter_BP` _returnvalue_2))
    (set `/Game/Characters/MyCharacter_BP.stopMovement` true _asmy_character_bp)
    (else
      (`Widget.RemoveFromParent` _doorcode_wid)
      (`WidgetBlueprintLibrary.SetInputMode_GameOnly` _returnvalue)
      (set `self.bShowMouseCursor` false)
      (bind _asmy_character_bp_2 (cast `/Game/Characters/MyCharacter_BP` _returnvalue_2))
      (set `/Game/Characters/MyCharacter_BP.stopMovement` false _asmy_character_bp_2))))

(event `ShowTemporalMessage`
  (params (messageText :type String) (delayMessage :type "Float (double-precision)"))
  (bind _temporalmessage_wid (`self.temporalMessage_WID`))
  (if (not (`Widget.IsInViewport` _temporalmessage_wid))
    (set `/Game/Interface/temporalMessage.delayMessage` delayMessage _temporalmessage_wid)
    (set `/Game/Interface/temporalMessage.messageText` messageText _temporalmessage_wid)
    (`UserWidget.AddToViewport` _temporalmessage_wid 0)))

(event `InputAction|OpenMenu`
  (params (Key :type "Key Structure"))
  (:`Pressed`
    (if (not (`self.openedExitMenu`))
      (`self.setStatusExitMenu` true))))

(event `Restart`
  (bind _returnvalue (`GameplayStatics.GetPlayerPawn` 0))
  (`WidgetBlueprintLibrary.SetInputMode_GameOnly` (`GameplayStatics.GetPlayerController` 0))
  (set `self.bShowMouseCursor` false)
  (bind _asmy_character_bp (cast `/Game/Characters/MyCharacter_BP` _returnvalue)
    (:`then`
      (set `/Game/Characters/MyCharacter_BP.stopMovement` false _asmy_character_bp))
    (:`CastFailed`
      (cast `/Game/Characters/MyCharacter_Soul_BP` _returnvalue)))
  (`GameplayStatics.SetGamePaused` false)
  (bind _returnvalue_2 (`GameplayStatics.GetCurrentLevelName` true))
  (`GameplayStatics.OpenLevel` (`KismetStringLibrary.Conv_StringToName` _returnvalue_2)))

(event `setStatusExitMenu`
  (params (openedExitMenu :type Boolean))
  (bind _returnvalue (`GameplayStatics.GetPlayerController` 0))
  (bind _returnvalue_2 (`GameplayStatics.GetPlayerPawn` 0))
  (bind _exitemenu (`self.exiteMenu`))
  (if openedExitMenu
    (`UserWidget.AddToViewport` _exitemenu 0)
    (`WidgetBlueprintLibrary.SetInputMode_UIOnlyEx` _returnvalue _exitemenu)
    (set `self.bShowMouseCursor` true)
    (bind _asmy_character_bp (cast `/Game/Characters/MyCharacter_BP` _returnvalue_2))
    (set `/Game/Characters/MyCharacter_BP.stopMovement` true _asmy_character_bp)
    (`GameplayStatics.SetGamePaused` true)
    (else
      (`Widget.RemoveFromParent` _exitemenu)
      (`WidgetBlueprintLibrary.SetInputMode_GameOnly` _returnvalue)
      (set `self.bShowMouseCursor` false)
      (bind _asmy_character_bp_2 (cast `/Game/Characters/MyCharacter_BP` _returnvalue_2))
      (set `/Game/Characters/MyCharacter_BP.stopMovement` false _asmy_character_bp_2)
      (`GameplayStatics.SetGamePaused` false)))
  (set `self.openedExitMenu` openedExitMenu))

(fn `UserConstructionScript`)