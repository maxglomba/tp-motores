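; Footstep actor that shows a temporary footprint on a Plane mesh.
; On BeginPlay it sets the plane's visibility from its Visibility variable through the setStepVisibility event.
; It then ages on timed delays, swapping to a second material halfway through its thirty-second life and destroying itself at the end.
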(event `self.ReceiveBeginPlay`
  (`self.setStepVisibility` (`self.visibility`))
  (`KismetSystemLibrary.Delay` 15.0)
  (`PrimitiveComponent.SetMaterial` (`self.Plane`) 0 "/Game/Materials/footStep_MAT2.footStep_MAT2")
  (`KismetSystemLibrary.Delay` 15.0)
  (`self.K2_DestroyActor`))

(event `setStepVisibility`
  (params (Visibility :type Boolean))
  (bind _plane (`self.Plane`))
  (if Visibility
    (`SceneComponent.SetVisibility` _plane true false)
    (else
      (`SceneComponent.SetVisibility` _plane false false))))

(fn `UserConstructionScript`)