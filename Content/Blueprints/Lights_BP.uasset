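; Light pickup actor that the soul character collects and that reveals ghosts near it.
; Collision is off from construction until five seconds after BeginPlay; a soul overlap then increments the body's Lights count once, plays a sound and destroys the actor.
; ShowGhostZone overlaps toggle ghost visibility only while the player pawn is MyCharacter_BP.
; A custom event shows or hides the Cylinder and its children.
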(event `self.ReceiveBeginPlay`
  (`KismetSystemLibrary.Delay` 5.0)
  (`self.SetActorEnableCollision` true))

(event `self.ReceiveActorBeginOverlap`
  (params (OtherActor :type "Actor Object Reference"))
  (bind _asmy_character_soul_bp (cast `/Game/Characters/MyCharacter_Soul_BP` OtherActor))
  (`/Engine/EditorBlueprintResources/StandardMacros.DoOnce` false
    (:`Completed`
      (bind _bodyref (`/Game/Characters/MyCharacter_Soul_BP.bodyRef` _asmy_character_soul_bp))
      (set `/Game/Characters/MyCharacter_BP.lights` (+ (`/Game/Characters/MyCharacter_BP.lights` _bodyref) 1) _bodyref)
      (`GameplayStatics.PlaySoundAtLocation` "/Game/Sounds/pickup_light.pickup_light" (`self.K2_GetActorLocation`) (struct) 1.0 1.0 0.0 null null null)
      (`self.K2_DestroyActor`))))

(event `SetVisibilityLight`
  (params (Visibility :type Boolean))
  (bind _cylinder (`self.Cylinder`))
  (if Visibility
    (`SceneComponent.SetVisibility` _cylinder true true)
    (else
      (`SceneComponent.SetVisibility` _cylinder false true))))

(event `self.ShowGhostZone.OnComponentBeginOverlap`
  (params (OverlappedComponent :type "PrimitiveComponent Object Reference") (OtherActor :type "Actor Object Reference") (OtherComp :type "PrimitiveComponent Object Reference") (OtherBodyIndex :type Integer) (bFromSweep :type Boolean) (SweepResult :type "HitResult Structure (by ref)"))
  (bind _asghost_bp (cast `/Game/IA/Enemies/Ghost/ghost_BP` OtherActor))
  (cast `/Game/Characters/MyCharacter_BP` (`GameplayStatics.GetPlayerPawn` 0))
  (`/Game/IA/Enemies/Ghost/ghost_BP.setGhostVisibility` _asghost_bp true))

(event `self.ShowGhostZone.OnComponentEndOverlap`
  (params (OverlappedComponent :type "PrimitiveComponent Object Reference") (OtherActor :type "Actor Object Reference") (OtherComp :type "PrimitiveComponent Object Reference") (OtherBodyIndex :type Integer))
  (bind _asghost_bp (cast `/Game/IA/Enemies/Ghost/ghost_BP` OtherActor))
  (cast `/Game/Characters/MyCharacter_BP` (`GameplayStatics.GetPlayerPawn` 0))
  (`/Game/IA/Enemies/Ghost/ghost_BP.setGhostVisibility` _asghost_bp false))

(fn `UserConstructionScript`
  (`self.SetActorEnableCollision` false))