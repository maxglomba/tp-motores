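; Game mode for a word-hint game with a toggleable "soul vision" that switches visibility of wall texts, footsteps and ghosts.
; PickWord randomly selects a word of length 2×Letters−1, or prints an error and possesses a spectator pawn when none match.
; The chain feeding the Hint actor count into PickWord is unconnected.
; SetTextHints hands out hint strings to wall actors through a wrapping index.
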(event `self.ReceiveBeginPlay`
  ;[0.2969 0 0] Begin Play
)

(event `Pick Word`
  (params (Letters :type Integer))
  (bind _returnvalue (`GameplayStatics.GetPlayerController` 0))
  ;[1 0.06152 0.2013] Pick Word From lenght and assign to current level word
  (bind _filteredwords (`self.FilterAvaibleWords` Letters))
  (bind _returnvalue_2 (`KismetArrayLibrary.Array_Length` _filteredwords))
  (if (> _returnvalue_2 0)
    (set `self.currentWord` (`|GetArrayItem` (`self.FilteredWords`) (`KismetMathLibrary.RandomIntegerInRange` 0 (- _returnvalue_2 1))))
    (else
      (`KismetSystemLibrary.PrintString` (`KismetStringLibrary.Concat_StrStr` "No se encontraron palabras con " (`KismetStringLibrary.Conv_IntToString` Letters) " letras"))
      (`Controller.UnPossess` _returnvalue)
      (bind _outactors (`GameplayStatics.GetAllActorsOfClass` "/Script/Engine.PlayerStart"))
      (bind _returnvalue_3 (`|SpawnActorFromClass` "/Script/Engine.SpectatorPawn" (`KismetMathLibrary.MakeTransform` (+ (`self.K2_GetActorLocation` (`|GetArrayItem` _outactors)) (0.0 0.0 200.0))) "Undefined" "OverrideRootScale" _returnvalue null))
      (`Controller.Possess` _returnvalue _returnvalue_3))))

(event `TurnSoulVision`
  (params (Enabled :type Boolean))
  (`self.Turn Walls Message` Enabled)
  (`self.Turn Footsteps` Enabled)
  (`self.Turn Ghosts` Enabled))

(fn `FilterAvaibleWords`
  (params (Letters :type Integer))
  (returns (FilteredWords :type "Array of String"))
  (for _array_element (`self.Words`)
    (if (== (`KismetStringLibrary.Len` _array_element) (- (* Letters 2) 1))
      (`KismetArrayLibrary.Array_Add` (`self.FilteredWords`) _array_element)))
  (return (`self.FilteredWords`)))

(fn `GetHints`
  (returns (Hints :type Integer))
  (bind _outactors (`GameplayStatics.GetAllActorsOfClass` "/Game/Blueprints/Hint.Hint_C"))
  (bind _output_get (set `self.wordLengh` (`KismetArrayLibrary.Array_Length` _outactors)))
  (return _output_get))

(fn `setTextHints`
  (params (wordHints :type "Array of String"))
  (bind _returnvalue (`KismetArrayLibrary.Array_Length` wordHints))
  (bind _outactors (`GameplayStatics.GetAllActorsOfClass` "/Game/Blueprints/HintWall_BP.HintWall_BP_C"))
  (if (and (> (`KismetArrayLibrary.Array_Length` _outactors) 0) (> _returnvalue 0))
    (for _array_element _outactors
      (bind _result (`/Engine/EditorBlueprintResources/StandardMacros.IncrementInt` (`self.lastUsedText`))
        (:`  `
          (bind _output_get (set `self.lastUsedText` _result))
          (if (> _output_get _returnvalue)
            (set `self.lastUsedText` 0))
          (`/Game/Blueprints/HintWall_BP.setTextHint` _array_element (`|GetArrayItem` wordHints (`self.lastUsedText`))))))))

(fn `Turn Footsteps`
  (params (Visible :type Boolean))
  (bind _outactors (`GameplayStatics.GetAllActorsOfClass` "/Game/Blueprints/footstep.footstep_C"))
  (if (> (`KismetArrayLibrary.Array_Length` _outactors) 0)
    (for _array_element _outactors
      (`/Game/Blueprints/footstep.setStepVisibility` _array_element Visible))))

(fn `Turn Ghosts`
  (params (visibility :type Boolean))
  (bind _outactors (`GameplayStatics.GetAllActorsOfClass` "/Game/IA/Enemies/Ghost/ghost_BP.ghost_BP_C"))
  (if (> (`KismetArrayLibrary.Array_Length` _outactors) 0)
    (for _array_element _outactors
      (`/Game/IA/Enemies/Ghost/ghost_BP.setGhostVisibility` _array_element visibility))))

(fn `Turn Walls Message`
  (params (Visible :type Boolean))
  (bind _outactors (`GameplayStatics.GetAllActorsOfClass` "/Game/Blueprints/HintWall_BP.HintWall_BP_C"))
  (if (> (`KismetArrayLibrary.Array_Length` _outactors) 0)
    (for _array_element _outactors
      (`/Game/Blueprints/HintWall_BP.SwitchTextVision` _array_element Visible))))

(fn `UserConstructionScript`)