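; Hint pickup actor that grants the player a missing letter of the current code word.
; When a non-Soul Player overlaps its sphere, it gathers the HUD's letters and compares them against the shuffled, underscore-split word from the game mode.
; The first missing letter is added to the HUD once, with a sound, and the actor is destroyed.
; If none is missing, it stays and shows a temporary Spanish message saying all letters are owned.
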(event `self.Sphere.OnComponentBeginOverlap`
  (params (OverlappedComponent :type "PrimitiveComponent Object Reference") (OtherActor :type "Actor Object Reference") (OtherComp :type "PrimitiveComponent Object Reference") (OtherBodyIndex :type Integer) (bFromSweep :type Boolean) (SweepResult :type "HitResult Structure (by ref)"))
  (if (and (`self.ActorHasTag` OtherActor "Player") (not (`self.ActorHasTag` OtherActor "Soul")))
    (bind _asmy_game_mode_bp (cast `/Game/Blueprints/MyGameMode_BP` (`GameplayStatics.GetGameMode`)))
    (bind _asmy_player_controller_bp (cast `/Game/Blueprints/MyPlayerController_BP` (`GameplayStatics.GetPlayerController` 0)))
    (set `self.AllLettersInventory` "")
    (for _array_element (`PanelWidget.GetAllChildren` (`/Game/Interface/HUD_WBP.Leters` (`/Game/Blueprints/MyPlayerController_BP.HUD` _asmy_player_controller_bp)))
      (bind _asletter_wbp (cast `/Game/Interface/Letter_WBP` _array_element))
      (set `self.AllLettersInventory` (`KismetStringLibrary.Concat_StrStr` (`self.AllLettersInventory`) (`/Game/Interface/Letter_WBP.Letter` _asletter_wbp))))
    (set `self.LettersWord` (`KismetStringLibrary.ParseIntoArray` (`/Game/Blueprints/MyGameMode_BP.currentWord` _asmy_game_mode_bp) "_"))
    (set `self.letterToAdd` "")
    (`KismetArrayLibrary.Array_Shuffle` (`self.LettersWord`))
    (for _array_element_2 (`self.LettersWord`)
      (if (not (> (`KismetStringLibrary.FindSubstring` (`self.AllLettersInventory`) _array_element_2) -1))
        (set `self.letterToAdd` _array_element_2)
        (break)))
    (if (> (`KismetStringLibrary.Len` (`self.letterToAdd`)) 0)
      (bind _asmy_player_controller_bp_2 (cast `/Game/Blueprints/MyPlayerController_BP` (`Pawn.GetController` (`GameplayStatics.GetPlayerPawn` 0))))
      (`/Engine/EditorBlueprintResources/StandardMacros.DoOnce` false
        (:`Completed`
          (`/Game/Interface/HUD_WBP.AddLetter` (`/Game/Blueprints/MyPlayerController_BP.HUD` _asmy_player_controller_bp_2) (`self.letterToAdd`))
          (`GameplayStatics.PlaySoundAtLocation` "/Game/Sounds/pickup_hint.pickup_hint" (`self.K2_GetActorLocation`) (struct) 1.0 1.0 0.0 null null null)
          (`self.K2_DestroyActor`)))
      (else
        (bind _asmy_player_controller_bp_3 (cast `/Game/Blueprints/MyPlayerController_BP` (`GameplayStatics.GetPlayerController` 0)))
        (`/Game/Blueprints/MyPlayerController_BP.ShowTemporalMessage` _asmy_player_controller_bp_3 "Tienes todas las letras del código!" 0.0)))))

(fn `UserConstructionScript`)